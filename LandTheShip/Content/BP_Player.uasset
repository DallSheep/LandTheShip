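; BP_Player is a physics-driven player actor that rolls left or right and thrusts along its up vector.
; BeginPlay adds the gameplay Enhanced Input mapping context, whose actions apply opposing world X-axis torque and upward-relative force to the static mesh.
; Tick fakes gravity with a velocity-change Z impulse every frame, not scaled by delta time.
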(event `self.ReceiveBeginPlay`
  (message `EnhancedInputSubsystemInterface.AddMappingContext` (pcsubsystem `EnhancedInputLocalPlayerSubsystem` (`GameplayStatics.GetPlayerController` 0)) "/Game/IMC_Gameplay.IMC_Gameplay" 0 (struct)))

(event `self.ReceiveTick`
  (params (DeltaSeconds :type "Float (single-precision)"))
  (`PrimitiveComponent.AddImpulse` (`self.StaticMesh`) (`KismetMathLibrary.MakeVector` 0.0 0.0 (`self.GravityStrength`)) "None" true) ; Spoofing Gravity (easier to work with)
)

(event `EnhancedInput|/Game/IA_RollLeft`
  (params (ActionValue :type Boolean) (ElapsedSeconds :type "Float (double-precision)") (TriggeredSeconds :type "Float (double-precision)") (InputAction :type "InputAction Object Reference" :default "/Game/IA_RollLeft.IA_RollLeft"))
  ;[1 1 1] Input
  (:`Triggered`
    (`PrimitiveComponent.AddTorqueInDegrees` (`self.StaticMesh`) (`KismetMathLibrary.MakeVector` (`self.RollStrength`)) "None" false)))

(event `EnhancedInput|/Game/IA_RollRight`
  (params (ActionValue :type Boolean) (ElapsedSeconds :type "Float (double-precision)") (TriggeredSeconds :type "Float (double-precision)") (InputAction :type "InputAction Object Reference" :default "/Game/IA_RollRight.IA_RollRight"))
  ;[1 1 1] Input
  (:`Triggered`
    (`PrimitiveComponent.AddTorqueInDegrees` (`self.StaticMesh`) (`KismetMathLibrary.MakeVector` (* (`self.RollStrength`) -1.0)) "None" false)))

(event `EnhancedInput|/Game/IA_Thrust`
  (params (ActionValue :type Boolean) (ElapsedSeconds :type "Float (double-precision)") (TriggeredSeconds :type "Float (double-precision)") (InputAction :type "InputAction Object Reference" :default "/Game/IA_Thrust.IA_Thrust"))
  ;[1 1 1] Input
  (:`Triggered`
    (`PrimitiveComponent.AddForce` (`self.StaticMesh`) (* (`self.GetActorUpVector`) (`self.ThrustStrength`)) "None" false)))

(fn `UserConstructionScript`)