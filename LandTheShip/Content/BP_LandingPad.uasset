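; BP_LandingPad is a landing pad that registers a landing once the player pawn has overlapped its Cube for over two seconds.
; Tick accumulates overlap time, which resets on exit, then Landed prints the BP_Gamemode timer and restarts the level, guarded by a DoOnce that resets after a delay.
; The construction script colors the pad by Difficulty, and RandomizeLocation moves it to a random Y at fixed X.
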(event `self.Cube.OnComponentBeginOverlap`
  (params (OverlappedComponent :type "PrimitiveComponent Object Reference") (OtherActor :type "Actor Object Reference") (OtherComp :type "PrimitiveComponent Object Reference") (OtherBodyIndex :type Integer) (bFromSweep :type Boolean) (SweepResult :type "HitResult Structure (by ref)"))
  (if (== OtherActor (`GameplayStatics.GetPlayerPawn` 0))
    (set `self.isOverlappingPlayer` true)))

(event `self.Cube.OnComponentEndOverlap`
  (params (OverlappedComponent :type "PrimitiveComponent Object Reference") (OtherActor :type "Actor Object Reference") (OtherComp :type "PrimitiveComponent Object Reference") (OtherBodyIndex :type Integer))
  (if (== OtherActor (`GameplayStatics.GetPlayerPawn` 0))
    (set `self.isOverlappingPlayer` false)
    (set `self.OverlappingPlayerDuration` 0.0)))

(event `self.ReceiveTick`
  (params (DeltaSeconds :type "Float (single-precision)"))
  (if (`self.isOverlappingPlayer`)
    (`KismetSystemLibrary.PrintString` "Landing..." true true (struct :`G` 0.66 :`B` 1.0 :`A` 1.0) 0.0)
    (bind _output_get (set `self.OverlappingPlayerDuration` (+ (`self.OverlappingPlayerDuration`) DeltaSeconds)))
    (if (> _output_get 2.0)
      (`self.Landed`))))

(event `Landed`
  (`/Engine/EditorBlueprintResources/StandardMacros.DoOnce` false :!label _label
    (:`Completed`
      (bind _asbp_gamemode (cast `/Game/BP_Gamemode` (`GameplayStatics.GetGameMode`)))
      (`KismetSystemLibrary.PrintString` (`KismetStringLibrary.Concat_StrStr` "Landed in " (`KismetStringLibrary.Conv_DoubleToString` (`/Game/Nick/WBP_Timer.Time` (`/Game/BP_Gamemode.TimerRef` _asbp_gamemode))) " Seconds!"))
      (`/Game/BP_Gamemode.RestartLevel` _asbp_gamemode)
      ;[1 0.02829 0] Delete this in actual game
      (`KismetSystemLibrary.Delay` 1.0)
      (goto _label :!via `Reset`))))

(fn `RandomizeLocation`
  (`self.K2_SetActorLocation` (`KismetMathLibrary.MakeVector` 810.0 (`KismetMathLibrary.Conv_IntToDouble` (`KismetMathLibrary.RandomIntegerInRange` -850 850)))))

(fn `UserConstructionScript`
  (`MeshComponent.SetVectorParameterValueOnMaterials` (`self.Cube`) "Color" (`KismetMathLibrary.Conv_LinearColorToVector` (select `/Game/E_LandingDifficulty` (`self.Difficulty`) :`NewEnumerator0` (struct :`G` 1.0 :`B` 0.049962 :`A` 1.0) :`NewEnumerator1` (struct :`R` 1.0 :`G` 0.923239 :`A` 1.0) :`NewEnumerator2` (struct :`R` 1.0 :`G` 0.025257 :`A` 1.0) :!type "LinearColor Structure"))))