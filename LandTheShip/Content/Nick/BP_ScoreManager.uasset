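; Score manager that rates a landing by time, player health and landing difficulty, awarding up to five stars.
; CalculateScore derives time score from the WBP_Timer widget, health score from BP_Player and a fixed bonus from difficulty.
; The summed score passes through nested StarThresholds checks to set StarsEarned, with no assignment when only the fifth check fails.
; It then prints a debug breakdown and adds the results widget to the viewport.
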(event `CalculateScore`
  (params (LandingDifficulty :type "/Game/Nick/E_LandingDifficulty Enum" :default "NewEnumerator0"))
  (`|ExecutionSequence`
    (:`then_0`
      (bind _foundwidgets (`WidgetBlueprintLibrary.GetAllWidgetsOfClass` "/Game/Nick/WBP_Timer.WBP_Timer_C"))
      (set `self.TimeScore` (- (* (`self.TimePointMultiplier`) 150.0) (* (`/Game/Nick/WBP_Timer.Time` (`|GetArrayItem` _foundwidgets)) 1.4))))
    (:`then_1`
      (bind _asbp_player (cast `/Game/Nick/BP_Player` (`GameplayStatics.GetPlayerPawn` 0)))
      (set `self.MaxHealth` (`/Game/Nick/BP_Player.MaxHealth` _asbp_player))
      (set `self.RemainingHealth` (`/Game/Nick/BP_Player.Health` _asbp_player))
      (set `self.HealthScore` (`KismetMathLibrary.Conv_IntToDouble` (- (* (`self.MaxHealth`) 100) (* (- (`self.MaxHealth`) (`self.RemainingHealth`)) 100)))))
    (:`then_2`
      (bind _output_get (set `self.LandingDifficulty` LandingDifficulty))
      (set `self.LandingScore` (select `/Game/Nick/E_LandingDifficulty` (cast `/Game/Nick/E_LandingDifficulty` _output_get) :`NewEnumerator0` 100.0 :`NewEnumerator1` 200.0 :`NewEnumerator2` 300.0)))
    (:`then_3`
      (bind _output_get_2 (set `self.FinalScore` (+ (`self.TimeScore`) (`self.HealthScore`) (`self.LandingScore`))))
      (if (> _output_get_2 (`BlueprintMapLibrary.Map_Find` (`self.StarThresholds`) 1))
        (if (> (`self.FinalScore`) (`BlueprintMapLibrary.Map_Find` (`self.StarThresholds`) 2))
          (if (> (`self.FinalScore`) (`BlueprintMapLibrary.Map_Find` (`self.StarThresholds`) 3))
            (if (> (`self.FinalScore`) (`BlueprintMapLibrary.Map_Find` (`self.StarThresholds`) 4))
              (if (> (`self.FinalScore`) (`BlueprintMapLibrary.Map_Find` (`self.StarThresholds`) 5))
                (set `self.StarsEarned` 5))
              (else
                (set `self.StarsEarned` 4)))
            (else
              (set `self.StarsEarned` 3)))
          (else
            (set `self.StarsEarned` 2)))
        (else
          (set `self.StarsEarned` 1)))
      (`KismetSystemLibrary.PrintString` (`KismetStringLibrary.Concat_StrStr` "TimeScore: " (`KismetStringLibrary.Conv_DoubleToString` (`self.TimeScore`)) "| HealthScore: " (`KismetStringLibrary.Conv_DoubleToString` (`self.HealthScore`)) "| LandingScore: " (`KismetStringLibrary.Conv_DoubleToString` (`self.LandingScore`)) "| FinalScore: " (`KismetStringLibrary.Conv_DoubleToString` (`self.FinalScore`)) "| StarsEarned: " (`KismetStringLibrary.Conv_IntToString` (`self.StarsEarned`))) true true (struct :`G` 0.66 :`B` 1.0 :`A` 1.0) 1000.0)
      (bind _returnvalue (`|CreateWidget` "/Game/UI/Wigets/ResultsWidget.ResultsWidget_C"))
      (`UserWidget.AddToViewport` _returnvalue 0))))

(fn `UserConstructionScript`)