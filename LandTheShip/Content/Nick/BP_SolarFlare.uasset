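; BP_SolarFlare is a recurring hazard that periodically warns of and then damages the player inside its volume.
; A looping timer plays a warning timeline that drives a Fade material parameter on the Cube mesh.
; When the timeline finishes, it resets the fade and calls TakeDamage on BP_Player if the player pawn overlaps the Cube at that moment.
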(event `self.ReceiveBeginPlay`
  (`KismetSystemLibrary.K2_SetTimer` null "WarnPlayer" 10.0 true))

(event `WarnPlayer`
  (bind (_direction _newtrack_0) (`Timeline|Timeline_Warning` :!via `PlayFromStart`)
    (:`Update`
      (`MeshComponent.SetScalarParameterValueOnMaterials` (`self.Cube`) "Fade" _newtrack_0))
    (:`Finished`
      (`self.TriggerDamage`))))

(event `TriggerDamage`
  (bind _returnvalue (`GameplayStatics.GetPlayerPawn` 0))
  (`MeshComponent.SetScalarParameterValueOnMaterials` (`self.Cube`) "Fade" -1.0)
  (if (`PrimitiveComponent.IsOverlappingActor` (`self.Cube`) _returnvalue)
    (bind _asbp_player (cast `/Game/Nick/BP_Player` _returnvalue))
    (`/Game/Nick/BP_Player.TakeDamage` _asbp_player)))

(fn `UserConstructionScript`)