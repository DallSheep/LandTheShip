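; Player ship pawn flown on physics with thrust and roll, limited by fuel and health.
; Enhanced Input drives force and torque on the mesh with thruster audio and effects, while Tick fakes gravity with a tunable impulse.
; Hard hits, thresholded by whether an asteroid is struck, cost health through a DoOnce cooldown and restart the level at zero.
; It also opens the pause menu, halts the HUD timer, and includes fuel and gravity debug keys.
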(event Custom|TakeDamage
  (Utilities|FlowControl|DoOnce false :!label _label
    (:Completed
      (bind _result (Math|Integer|DecrementInt (Variables|Default|GetHealth)) ; Reduce Health
        (:%20%20
          (Development|PrintString (Utilities|String|Append "Health Remaining: " (Utilities|String|ToString(Integer) _result)))
          (if (<= (Variables|Default|GetHealth) 0) ; is player dead?
            (Audio|PlaySoundatLocation (.OutItem (Utilities|Array|Random (Utilities|Array|MakeArray "/Game/Michael_Audio/Audio_Files/Ship_Explosion-001.Ship_Explosion-001" "/Game/Michael_Audio/Audio_Files/Ship_Explosion-002.Ship_Explosion-002" "/Game/Michael_Audio/Audio_Files/Ship_Explosion-003.Ship_Explosion-003" "/Game/Michael_Audio/Audio_Files/Ship_Explosion-004.Ship_Explosion-004" "/Game/Michael_Audio/Audio_Files/Ship_Explosion-005.Ship_Explosion-005" "/Game/Michael_Audio/Audio_Files/Ship_Explosion-006.Ship_Explosion-006"))) (Transformation|GetActorLocation) "0, 0, 0" 4.0 1.0 0.0 0 0 0 0)
            (Utilities|FlowControl|Delay 2.0)
            (bind _asbp_gamemode (Utilities|Casting|CastToBP_Gamemode (Game|GetGameMode)))
            (Default|RestartLevel _asbp_gamemode)
            (else
              (Utilities|FlowControl|Delay 1.0)
              (goto _label Reset))))))))

(event Custom|DecayThrustRecency
  ;[1 1 1] Input
  (Variables|Default|SetThrustRecency (Math|Float|Max(Float) (- (Variables|Default|GetThrustRecency) 0.2) 0.0)))

(event Input|EnhancedActionEvents|EnhancedInputActionIA_RollLeft
  (params (ActionValue :type Boolean) (ElapsedSeconds :type Float%20%28double-precision%29) (TriggeredSeconds :type Float%20%28double-precision%29) (InputAction :type Input%20Action%20Object%20Reference :default "/Game/Nick/IA_RollLeft.IA_RollLeft"))
  ;[1 1 1] Input
  (:Triggered
    (Class|PrimitiveComponent|AddTorqueinDegrees (Variables|Default|GetStaticMesh) (Math|Vector|MakeVector (Variables|Default|GetRollStrength) 0.0 0.0) "None" false))
  (:Started
    (bind _returnvalue (Audio|SpawnSound2D "/Game/Michael_Audio/MS_SideThrusters.MS_SideThrusters" 1.0 1.0 0.0 0)))
  (:Completed
    (Class|AudioParameterControllerInterface|SetTriggerParameter _returnvalue "Thruster Stop")))

(event Input|EnhancedActionEvents|EnhancedInputActionIA_Thrust
  (params (ActionValue :type Boolean) (ElapsedSeconds :type Float%20%28double-precision%29) (TriggeredSeconds :type Float%20%28double-precision%29) (InputAction :type Input%20Action%20Object%20Reference :default "/Game/Nick/IA_Thrust.IA_Thrust"))
  ;[1 1 1] Input
  (:Triggered
    (if (> (Variables|Default|GetRemainingFuel) 0.0)
      (Components|Activation|Activate (Variables|Default|GetNiagara) false)
      (Physics|AddForce (Variables|Default|GetStaticMesh) (* (Transformation|GetActorUpVector) (Variables|Default|GetThrustStrength)) "None" false)
      (bind _output_get (Variables|Default|SetRemainingFuel (- (Variables|Default|GetRemainingFuel) 0.5)))
      (Development|PrintString (Utilities|String|Append "Fuel: " (Utilities|String|ToString(Float) _output_get)) true true "(R=0.000000,G=0.660000,B=1.000000,A=1.000000)" 0.0)
      (else
        (Development|PrintString "Out of Fuel!" true true "(R=0.000000,G=0.660000,B=1.000000,A=1.000000)" 0.0)
        (Components|Activation|Deactivate (Variables|Default|GetNiagara)))))
  (:Started
    (bind _returnvalue (Audio|SpawnSound2D "/Game/Michael_Audio/MS_Thrusters.MS_Thrusters" (- 1.0 (Variables|Default|GetThrustRecency)) 1.0 0.0 0))
    (Variables|Default|SetThrustRecency (Math|Float|Min(Float) (+ (Variables|Default|GetThrustRecency) 0.1) 0.6))
    (Utilities|Time|SetTimerbyFunctionName 0 "DecayThrustRecency" 0.5))
  (:Completed
    (Components|Activation|Deactivate (Variables|Default|GetNiagara))
    (Class|AudioParameterControllerInterface|SetTriggerParameter _returnvalue "Thruster Stop")))

(event Input|EnhancedActionEvents|EnhancedInputActionIA_RollRight
  (params (ActionValue :type Boolean) (ElapsedSeconds :type Float%20%28double-precision%29) (TriggeredSeconds :type Float%20%28double-precision%29) (InputAction :type Input%20Action%20Object%20Reference :default "/Game/Nick/IA_RollRight.IA_RollRight"))
  ;[1 1 1] Input
  (:Triggered
    (Class|PrimitiveComponent|AddTorqueinDegrees (Variables|Default|GetStaticMesh) (Math|Vector|MakeVector (* (Variables|Default|GetRollStrength) -1.0) 0.0 0.0) "None" false))
  (:Started
    (bind _returnvalue (Audio|SpawnSound2D "/Game/Michael_Audio/MS_SideThrusters.MS_SideThrusters" 1.0 1.0 0.0 0)))
  (:Completed
    (Class|AudioParameterControllerInterface|SetTriggerParameter _returnvalue "Thruster Stop")))

(event Input|EnhancedActionEvents|EnhancedInputActionIA_Pause
  (params (ActionValue :type Boolean) (ElapsedSeconds :type Float%20%28double-precision%29) (TriggeredSeconds :type Float%20%28double-precision%29) (InputAction :type Input%20Action%20Object%20Reference :default "/Game/IA_Pause.IA_Pause"))
  (bind _returnvalue (Game|GetPlayerController 0))
  ;[1 1 1] Input
  (Game|SetGamePaused true)
  (bind _returnvalue_2 (UserInterface|CreateWidget "/Game/UI/Wigets/WBP_Pause.WBP_Pause_C"))
  (UserInterface|Viewport|AddtoViewport _returnvalue_2 0)
  (Input|SetInputModeUIOnly _returnvalue _returnvalue_2 "DoNotLock" true)
  (Variables|/Script/Engine.PlayerController|SetbShowMouseCursor _returnvalue true)
  (Variables|/Game/Nick/WBP_Timer.WBP_Timer_C|SetisTimerGoing (Variables|Default|GetHUDRef) false))

(event EventTick
  (params (DeltaSeconds :type Float%20%28single-precision%29))
  (Physics|AddImpulse (Variables|Default|GetStaticMesh) (Math|Vector|MakeVector 0.0 0.0 (Variables|Default|GetGravityStrength)) "None" true) ; Spoofing Gravity (easier to work with)
)

(event Collision|EventHit
  (params (MyComp :type Primitive%20Component%20Object%20Reference) (Other :type Actor%20Object%20Reference) (OtherComp :type Primitive%20Component%20Object%20Reference) (bSelfMoved :type Boolean) (HitLocation :type Vector :default "0, 0, 0") (HitNormal :type Vector :default "0, 0, 0") (NormalImpulse :type Vector :default "0, 0, 0") (Hit :type Hit%20Result%20Structure%20%28by%20ref%29))
  (bind _returnvalue (Math|Vector|VectorLength NormalImpulse))
  (if (> _returnvalue (Math|Float|SelectFloat 7e+03 1e+04 (== (Utilities|GetClass Other) "/Game/Obstacles/BP_Asteriod.BP_Asteriod_C")))
    (CallFunction|TakeDamage)
    (Audio|PlaySoundatLocation (.OutItem (Utilities|Array|Random (Utilities|Array|MakeArray "/Game/Michael_Audio/Audio_Files/Ship_Impacts-001.Ship_Impacts-001" "/Game/Michael_Audio/Audio_Files/Ship_Impacts-002.Ship_Impacts-002" "/Game/Michael_Audio/Audio_Files/Ship_Impacts-003.Ship_Impacts-003" "/Game/Michael_Audio/Audio_Files/Ship_Impacts-004.Ship_Impacts-004" "/Game/Michael_Audio/Audio_Files/Ship_Impacts-005.Ship_Impacts-005"))) (Transformation|GetActorLocation) "0, 0, 0" 0.5 1.0 0.0 0 0 0 0)
    (elif (> _returnvalue 1e+03)
      (Audio|PlaySoundatLocation (.OutItem (Utilities|Array|Random (Utilities|Array|MakeArray "/Game/Michael_Audio/Audio_Files/Ship_Minor_Hits-001.Ship_Minor_Hits-001" "/Game/Michael_Audio/Audio_Files/Ship_Minor_Hits-002.Ship_Minor_Hits-002" "/Game/Michael_Audio/Audio_Files/Ship_Minor_Hits-003.Ship_Minor_Hits-003" "/Game/Michael_Audio/Audio_Files/Ship_Minor_Hits-004.Ship_Minor_Hits-004" "/Game/Michael_Audio/Audio_Files/Ship_Minor_Hits-005.Ship_Minor_Hits-005" "/Game/Michael_Audio/Audio_Files/Ship_Minor_Hits-006.Ship_Minor_Hits-006"))) (Transformation|GetActorLocation) "0, 0, 0" 0.5 1.0 0.0 0 0 0 0))))

(event EventBeginPlay
  (Input|AddMappingContext (PlayerController|LocalPlayerSubsystems|GetEnhancedInputLocalPlayerSubsystem (Game|GetPlayerController 0)) "/Game/Nick/IMC_Gameplay.IMC_Gameplay" 0 "(bIgnoreAllPressedKeysUntilRelease=True,bForceImmediately=False,bNotifyUserSettings=False)")
  (Variables|Default|SetRemainingFuel (Variables|Default|GetMaxFuel))
  (Variables|Default|SetHealth (Variables|Default|GetMaxHealth))
  (bind _foundwidgets (Widget|GetAllWidgetsOfClass "/Game/Nick/WBP_Timer.WBP_Timer_C" true))
  (Variables|Default|SetHUDRef (Utilities|Array|Get(acopy) _foundwidgets)))

(event Input|KeyboardEvents|DebugKeyF
  (params (Key :type Key%20Structure :default "None") (ActionValue :type Input%20Action%20Value%20Structure))
  ;[1 0.8869 0] Debug Inputs
  (:Pressed
    (Variables|Default|SetRemainingFuel (+ (Variables|Default|GetRemainingFuel) 3e+01))))

(event Input|KeyboardEvents|DebugKeyAdd
  (params (Key :type Key%20Structure :default "None") (ActionValue :type Input%20Action%20Value%20Structure))
  ;[1 0.8869 0] Debug Inputs
  (:Pressed
    (Variables|Default|SetGravityStrength (- (Variables|Default|GetGravityStrength) 0.2))))

(event Input|KeyboardEvents|DebugKeySubtract
  (params (Key :type Key%20Structure :default "None") (ActionValue :type Input%20Action%20Value%20Structure))
  ;[1 0.8869 0] Debug Inputs
  (:Pressed
    (Variables|Default|SetGravityStrength (+ (Variables|Default|GetGravityStrength) 0.2))))

(fn ConstructionScript)