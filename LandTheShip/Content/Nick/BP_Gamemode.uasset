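; Game mode for a landing game that sets the level camera as the view, creates the timer widget and handles level restarts.
; Each tick the camera follows the player's height, clamped so it never drops below a TargetPoint marking the bottom.
; RestartLevel reloads LVL_GameLevel1; an in-place reset of player, landing pad, gravity and timer remains in the graph but is disconnected.
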(event `self.ReceiveBeginPlay`
  (bind _returnvalue (`GameplayStatics.GetActorOfClass` "/Script/Engine.CameraActor"))
  (set `self.CameraRef` _returnvalue)
  (`PlayerController.SetViewTargetWithBlend` (`GameplayStatics.GetPlayerController` 0) (`self.CameraRef`) 0.0 "VTBlend_Linear" 0.0 false)
  (bind _asbp_player (cast `/Game/Nick/BP_Player` (`GameplayStatics.GetPlayerPawn` 0)))
  (set `self.PlayerRef` _asbp_player)
  (bind _returnvalue_2 (`|CreateWidget` "/Game/Nick/WBP_Timer.WBP_Timer_C"))
  (bind _output_get (set `self.TimerRef` _returnvalue_2))
  (`UserWidget.AddToViewport` _output_get 0)
  (bind _returnvalue_3 (`GameplayStatics.GetActorOfClass` "/Script/Engine.TargetPoint"))
  (bind (_returnvalue_x _returnvalue_y _returnvalue_z) (`KismetMathLibrary.BreakVector` (`self.K2_GetActorLocation` _returnvalue_3)))
  (set `self.BottomLevelZ` _returnvalue_z))

(event `self.ReceiveTick`
  (params (DeltaSeconds :type "Float (single-precision)"))
  (bind _cameraref (`self.CameraRef`))
  (bind (_returnvalue_x _returnvalue_y _returnvalue_z) (`KismetMathLibrary.BreakVector` (`self.K2_GetActorLocation` (`self.PlayerRef`))))
  (bind (_returnvalue_x_2 _returnvalue_y_2) (`KismetMathLibrary.BreakVector` (`self.K2_GetActorLocation` _cameraref)))
  (`self.K2_SetActorLocation` _cameraref (`KismetMathLibrary.MakeVector` _returnvalue_x_2 _returnvalue_y_2 (`KismetMathLibrary.FMax` _returnvalue_z (`self.BottomLevelZ`))) false false))

(event `RestartLevel`
  (`GameplayStatics.OpenLevelBySoftObjectPtr` "/Game/LVL_GameLevel1.LVL_GameLevel1"))

(fn `SendPlayerBackToStart`
  (bind _staticmesh (`/Game/Nick/BP_Player.StaticMesh` (`self.PlayerRef`)))
  (bind _returnvalue (`GameplayStatics.GetActorOfClass` "/Script/Engine.PlayerStart"))
  (bind (_returnvalue_location _returnvalue_rotation) (`KismetMathLibrary.BreakTransform` (`self.GetTransform` _returnvalue)))
  (`self.K2_SetActorLocationAndRotation` (`self.PlayerRef`) _returnvalue_location _returnvalue_rotation false false)
  (`PrimitiveComponent.SetPhysicsLinearVelocity` _staticmesh (0.0 0.0 0.0) false "None")
  (`PrimitiveComponent.SetPhysicsAngularVelocityInDegrees` _staticmesh (0.0 0.0 0.0) false "None"))

(fn `UserConstructionScript`)