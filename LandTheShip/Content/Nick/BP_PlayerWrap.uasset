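; BP_PlayerWrap is an actor that wraps player 0 to the opposite side along Y when it leaves a Box volume.
; Each Tick polls the Box overlap and, on exit, teleports the pawn just inside the far edge, keeping X and Z.
; The side's sign multiplies actor Y plus the inset extent, so placement is correct only with the actor at world Y zero.
; The end-overlap event is empty.
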(event `self.ReceiveTick`
  (params (DeltaSeconds :type "Float (single-precision)"))
  (bind _returnvalue (`GameplayStatics.GetPlayerPawn` 0))
  (bind (_returnvalue_x _returnvalue_y) (`KismetMathLibrary.BreakVector` (`self.K2_GetActorLocation`)))
  (bind (_returnvalue_x_2 _returnvalue_y_2 _returnvalue_z) (`KismetMathLibrary.BreakVector` (`self.K2_GetActorLocation` _returnvalue)))
  (bind (_boxextent_x _boxextent_y) (`KismetMathLibrary.BreakVector` (`BoxComponent.BoxExtent` (`self.Box`))))
  (if (not (`PrimitiveComponent.IsOverlappingActor` (`self.Box`) (`GameplayStatics.GetPlayerPawn` 0)))
    (`KismetSystemLibrary.PrintString` "Player Left")
    (`self.K2_SetActorLocation` _returnvalue (`KismetMathLibrary.MakeVector` _returnvalue_x_2 (`KismetMathLibrary.Conv_IntToDouble` (* (- (* (`KismetMathLibrary.Conv_BoolToInt` (< _returnvalue_y_2 _returnvalue_y)) 2) 1) (+ _returnvalue_y (- _boxextent_y 100.0)))) _returnvalue_z) false true)))

(event `self.Box.OnComponentEndOverlap`
  (params (OverlappedComponent :type "PrimitiveComponent Object Reference") (OtherActor :type "Actor Object Reference") (OtherComp :type "PrimitiveComponent Object Reference") (OtherBodyIndex :type Integer)))

(fn `UserConstructionScript`)