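; Game mode for a physics-driven landing game that sets up the camera, player reference and timer widget.
; BeginPlay switches the view to a level camera, which Tick moves to match the player's height only.
; RestartLevel returns the player to PlayerStart with zeroed velocities, resets health and timer, randomizes the landing pad location and rolls a new gravity strength.
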(event `self.ReceiveBeginPlay`
  (bind _returnvalue (`GameplayStatics.GetActorOfClass` "/Script/Engine.CameraActor"))
  (set `self.CameraRef` _returnvalue)
  (`PlayerController.SetViewTargetWithBlend` (`GameplayStatics.GetPlayerController` 0) (`self.CameraRef`) 0.0 "VTBlend_Linear" 0.0 false)
  (bind _asbp_player (cast `/Game/BP_Player` (`GameplayStatics.GetPlayerPawn` 0)))
  (set `self.PlayerRef` _asbp_player)
  (bind _returnvalue_2 (`|CreateWidget` "/Game/Nick/WBP_Timer.WBP_Timer_C"))
  (bind _output_get (set `self.TimerRef` _returnvalue_2))
  (`UserWidget.AddToViewport` _output_get 0))

(event `self.ReceiveTick`
  (params (DeltaSeconds :type "Float (single-precision)"))
  (bind _cameraref (`self.CameraRef`))
  (bind (_returnvalue_x _returnvalue_y _returnvalue_z) (`KismetMathLibrary.BreakVector` (`self.K2_GetActorLocation` (`self.PlayerRef`))))
  (bind (_returnvalue_x_2 _returnvalue_y_2) (`KismetMathLibrary.BreakVector` (`self.K2_GetActorLocation` _cameraref)))
  ;[1 1 1] Camera Follows Player Z
  (`self.K2_SetActorLocation` _cameraref (`KismetMathLibrary.MakeVector` _returnvalue_x_2 _returnvalue_y_2 _returnvalue_z) false false))

(event `RestartLevel`
  (bind _playerref (`self.PlayerRef`))
  (`self.SendPlayerBackToStart`)
  (set `/Game/BP_Player.Health` (defaults `Object` (`GameplayStatics.GetObjectClass` _playerref)) _playerref) ; Reset player health
  (bind _returnvalue (`GameplayStatics.GetActorOfClass` "/Game/BP_LandingPad.BP_LandingPad_C"))
  (`/Game/BP_LandingPad.RandomizeLocation` _returnvalue)
  ;[1 1 1] Randomize Gravity
  (bind _output_get (set `/Game/BP_Player.GravityStrength` (`KismetMathLibrary.RandomFloatInRange` -2.0 -5.0) (`self.PlayerRef`)))
  (`KismetSystemLibrary.PrintString` (`KismetStringLibrary.Concat_StrStr` "New Graivty Strength: " (`KismetStringLibrary.Conv_DoubleToString` _output_get)))
  (`/Game/Nick/WBP_Timer.Reset` (`self.TimerRef`)))

(fn `SendPlayerBackToStart`
  (bind _staticmesh (`/Game/BP_Player.StaticMesh` (`self.PlayerRef`)))
  (bind _returnvalue (`GameplayStatics.GetActorOfClass` "/Script/Engine.PlayerStart"))
  (bind (_returnvalue_location _returnvalue_rotation) (`KismetMathLibrary.BreakTransform` (`self.GetTransform` _returnvalue)))
  (`self.K2_SetActorLocationAndRotation` (`self.PlayerRef`) _returnvalue_location _returnvalue_rotation false false)
  (`PrimitiveComponent.SetPhysicsLinearVelocity` _staticmesh (0.0 0.0 0.0) false "None")
  (`PrimitiveComponent.SetPhysicsAngularVelocityInDegrees` _staticmesh (0.0 0.0 0.0) false "None"))

(fn `UserConstructionScript`)