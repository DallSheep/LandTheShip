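; BP_StationaryObstacle is an obstacle actor whose static mesh rotates in place.
; The construction script applies a configurable mesh and scale.
; On BeginPlay it starts the TL_RotateObject timeline and picks a random target rotation from RotationArr.
; Each timeline update lerps the mesh's relative rotation toward that target using the timeline alpha.
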(event `self.ReceiveBeginPlay`
  (`self.PlayTimeline`)
  (set `self.BaseRotationB` (`KismetArrayLibrary.Array_Random` (`self.RotationArr`))))

(event `PlayTimeline`
  (bind (_direction _alpha) (`Timeline|TL_RotateObject`)
    (:`Update`
      (`SceneComponent.K2_SetRelativeRotation` (`self.Static_Mesh`) (`KismetMathLibrary.RLerp` (struct) (`self.BaseRotationB`) _alpha) false false))))

(fn `UserConstructionScript`
  (`StaticMeshComponent.SetStaticMesh` (`self.Static_Mesh`) (`self.NewMesh`))
  (`SceneComponent.SetRelativeScale3D` (`self.Static_Mesh`) (`KismetMathLibrary.Conv_DoubleToVector` (`self.StaticMeshScale`))))