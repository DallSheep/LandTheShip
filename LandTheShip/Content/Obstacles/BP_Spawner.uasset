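; BP_Spawner is an obstacle spawner that periodically creates BP_Asteriod actors.
; On BeginPlay it caches the BP_Player pawn, stopping if the cast fails, then starts a looping timer on SpawnAsteriod.
; Each tick of that timer spawns an asteroid at fixed X with random Y and Z.
; It also re-randomizes SpawnTime, but the timer is never reset, so the running interval stays unchanged.
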(event `self.ReceiveBeginPlay`
  (bind _asbp_player (cast `/Game/BP_Player` (`GameplayStatics.GetPlayerPawn` 0)))
  (set `self.Player_Ref` _asbp_player)
  (bind _returnvalue (`KismetSystemLibrary.K2_SetTimerDelegate` (delegate `SpawnAsteriod`) (`self.SpawnTime`) true))
  (set `self.SpawnAsteriodTimer_Ref` _returnvalue))

(event `SpawnAsteriod`
  (`|SpawnActorFromClass` "/Game/Obstacles/BP_Asteriod.BP_Asteriod_C" (`KismetMathLibrary.MakeTransform` (`KismetMathLibrary.MakeVector` 800.0 (`KismetMathLibrary.RandomFloatInRange` -1000.0 1000.0) (`KismetMathLibrary.RandomFloatInRange` 100.0 1000.0))) "Undefined" "MultiplyWithRoot" null null)
  (set `self.SpawnTime` (`KismetMathLibrary.RandomFloatInRange` 1.0 3.0)))

(fn `UserConstructionScript`)