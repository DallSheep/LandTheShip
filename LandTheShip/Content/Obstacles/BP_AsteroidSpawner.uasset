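; Asteroid spawner that periodically spawns one or two BP_Asteriod actors beyond the edges of a camera-relative rectangle.
; BeginPlay caches the player and CameraActor, then starts a looping SpawnAsteriod timer.
; Each spawn picks one of four sides from GetSpawnLocations, offset from the camera with random position along that edge, at fixed X depth.
; SpawnTime is re-randomized and printed afterwards, but the running timer keeps its initial interval.
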(event `self.ReceiveBeginPlay`
  (`|ExecutionSequence`
    (:`then_0`
      (bind _asbp_player (cast `/Game/Nick/BP_Player` (`GameplayStatics.GetPlayerPawn` 0)))
      (set `self.Player_Ref` _asbp_player)
      (bind _returnvalue (`GameplayStatics.GetActorOfClass` "/Script/Engine.CameraActor"))
      (set `self.Camera_Ref` _returnvalue))
    (:`then_1`
      (bind _returnvalue_2 (`KismetSystemLibrary.K2_SetTimerDelegate` (delegate `SpawnAsteriod`) (`KismetMathLibrary.Conv_IntToDouble` (`self.SpawnTime`)) true))
      (set `self.SpawnAsteriodTimer_Ref` _returnvalue_2))))

(event `SpawnAsteriod`
  (bind (_astroidspawnlocation_x _astroidspawnlocation_y _astroidspawnlocation_z) (`KismetMathLibrary.BreakVector` (`self.AstroidSpawnLocation`)))
  ;[0.2974 0.8188 1] Determines how many asteroids to spawn
  (for _ (range (+ (`KismetMathLibrary.RandomIntegerInRange` 1 2) 1))
    ;[0.2974 0.8188 1] Determines the spawn locations of the asteroids and spawns them
    (set `self.Spawn Points` (`KismetMathLibrary.RandomIntegerInRange` 0 3))
    (bind (_z_up _z_down _y_left _y_right) (`self.GetSpawnLocations`))
    (set `self.AstroidSpawnLocation` (select `int` (`self.Spawn Points`) :`0` _z_up :`1` _z_down :`2` _y_left :`3` _y_right))
    (`|SpawnActorFromClass` "/Game/Obstacles/BP_Asteriod.BP_Asteriod_C" (`KismetMathLibrary.MakeTransform` (`KismetMathLibrary.MakeVector` 800.0 _astroidspawnlocation_y _astroidspawnlocation_z)) "Undefined" "MultiplyWithRoot" null null))
  ;[1 0.7709 0] sets time till next spawn
  (bind _output_get (set `self.SpawnTime` (`KismetMathLibrary.RandomIntegerInRange` 4 5)))
  (`KismetSystemLibrary.PrintString` (`KismetStringLibrary.Conv_IntToString` _output_get)))

(fn `GetSpawnLocations`
  (returns (`Z-Up` :type "Vector Structure") (`Z-Down` :type "Vector Structure") (`Y-Left` :type "Vector Structure") (`Y-Right` :type "Vector Structure"))
  (bind (_returnvalue_x _returnvalue_y _returnvalue_z) (`KismetMathLibrary.BreakVector` (`self.K2_GetActorLocation` (`self.Camera_Ref`))))
  (bind (_returnvalue_x_2 _returnvalue_y_2) (`KismetMathLibrary.BreakVector` (`self.K2_GetActorLocation` (`self.Camera_Ref`))))
  (bind (_returnvalue_x_3 _returnvalue_y_3 _returnvalue_z_2) (`KismetMathLibrary.BreakVector` (`self.K2_GetActorLocation` (`self.Camera_Ref`))))
  (bind (_returnvalue_x_4 _returnvalue_y_4) (`KismetMathLibrary.BreakVector` (`self.K2_GetActorLocation` (`self.Camera_Ref`))))
  (`|ExecutionSequence`
    (:`then_0`
      (set `self.Z-Axis Up` (+ _returnvalue_z 1750.0)))
    (:`then_1`
      (set `self.Z-Axis Down` (+ _returnvalue_z_2 -1750.0)))
    (:`then_2`
      (set `self.Y-Axis Right` (+ _returnvalue_y_4 1000.0)))
    (:`then_3`
      (set `self.Y-Axis Left` (+ _returnvalue_y_2 -1000.0)))
    (:`then_4`
      (return (`KismetMathLibrary.MakeVector` 0.0 (`KismetMathLibrary.RandomFloatInRange` -1000.0 1000.0) (`self.Z-Axis Up`)) (`KismetMathLibrary.MakeVector` 0.0 (`KismetMathLibrary.RandomFloatInRange` -1000.0 1000.0) (`self.Z-Axis Down`)) (`KismetMathLibrary.MakeVector` 0.0 (`self.Y-Axis Left`) (`KismetMathLibrary.RandomFloatInRange` -1750.0 1750.0)) (`KismetMathLibrary.MakeVector` 0.0 (`self.Y-Axis Right`) (`KismetMathLibrary.RandomFloatInRange` -1750.0 1750.0))))))

(fn `UserConstructionScript`)