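; Asteroid obstacle that is pushed toward the player and damages it on contact.
; On BeginPlay it caches BP_Player and applies a one-off, mass-independent force to its mesh in the YZ plane.
; AstroidSpeed scales the unnormalized offset to the player by a random factor, so farther spawns get stronger pushes.
; Hitting the player calls its TakeDamage directly; an ApplyDamage node is left unconnected.
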(event `self.ReceiveBeginPlay`
  (`|ExecutionSequence`
    (:`then_0`
      (bind _returnvalue (`GameplayStatics.GetActorOfClass` "/Game/Nick/BP_Player.BP_Player_C"))
      (set `self.Player_Ref` _returnvalue))
    (:`then_1`
      (bind (_y _z) (`self.AstroidSpeed` 10.0 25.0))
      (`PrimitiveComponent.AddForce` (`self.SM_Asteriod`) (`KismetMathLibrary.MakeVector` 0.0 _y _z) "None" true))))

(event `self.ReceiveHit`
  (params (MyComp :type "PrimitiveComponent Object Reference") (Other :type "Actor Object Reference") (OtherComp :type "PrimitiveComponent Object Reference") (bSelfMoved :type Boolean) (HitLocation :type "Vector Structure") (HitNormal :type "Vector Structure") (NormalImpulse :type "Vector Structure") (Hit :type "HitResult Structure (by ref)"))
  (bind _player_ref (`self.Player_Ref`))
  (if (== Other _player_ref)
    (`/Game/Nick/BP_Player.TakeDamage` _player_ref)))

(fn `AstroidSpeed`
  (params (Min :type "Float (double-precision)") (Max :type "Float (double-precision)"))
  (returns (Y :type "Float (double-precision)") (Z :type "Float (double-precision)"))
  (bind _output_get (set `self.PlayerLocation` (`self.K2_GetActorLocation` (`self.Player_Ref`))))
  (return (.y (* (- _output_get (`self.K2_GetActorLocation`)) (`KismetMathLibrary.RandomFloatInRange` Min Max))) (.z (* (- _output_get (`self.K2_GetActorLocation`)) (`KismetMathLibrary.RandomFloatInRange` Min Max)))))

(fn `UserConstructionScript`)