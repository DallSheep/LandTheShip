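; BP_SFX_Master plays the thruster sounds in response to raw key input.
; A and D each spawn a 2D side-thruster sound and SpaceBar a main thruster sound, each sent a "Thruster Stop" trigger on release.
; Repeated SpaceBar presses raise a capped ThrustRecency value that quiets later spawns.
; A non-looping timer, reset on each press, lowers that value one step shortly after the last press.
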(event `Key|A`
  (params (Key :type "Key Structure"))
  ;[1 0.2614 0.5513] Thrusters
  (:`Pressed`
    (bind _returnvalue (`GameplayStatics.SpawnSound2D` "/Game/Michael_Audio/MS_SideThrusters.MS_SideThrusters" 1.0 1.0 0.0 null)))
  (:`Released`
    (`AudioParameterControllerInterface.SetTriggerParameter` _returnvalue "Thruster Stop")))

(event `Key|D`
  (params (Key :type "Key Structure"))
  ;[1 0.2614 0.5513] Thrusters
  (:`Pressed`
    (bind _returnvalue (`GameplayStatics.SpawnSound2D` "/Game/Michael_Audio/MS_SideThrusters.MS_SideThrusters" 1.0 1.0 0.0 null)))
  (:`Released`
    (`AudioParameterControllerInterface.SetTriggerParameter` _returnvalue "Thruster Stop")))

(event `Key|SpaceBar`
  (params (Key :type "Key Structure"))
  ;[1 0.2614 0.5513] Thrusters
  (:`Pressed`
    (bind _returnvalue (`GameplayStatics.SpawnSound2D` "/Game/Michael_Audio/MS_Thrusters.MS_Thrusters" (- 1.0 (`self.ThrustRecency`)) 1.0 0.0 null))
    (set `self.ThrustRecency` (`KismetMathLibrary.FMin` (+ (`self.ThrustRecency`) 0.1) 0.6))
    (`KismetSystemLibrary.K2_SetTimer` null "DecayThrustRecency" 0.5))
  (:`Released`
    (`AudioParameterControllerInterface.SetTriggerParameter` _returnvalue "Thruster Stop")))

(event `DecayThrustRecency`
  (set `self.ThrustRecency` (`KismetMathLibrary.FMax` (- (`self.ThrustRecency`) 0.2))))

(fn `UserConstructionScript`)