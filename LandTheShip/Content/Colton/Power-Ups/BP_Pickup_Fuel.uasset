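; BP_Pickup_Fuel is a fuel power-up that refills part of the player's fuel when picked up.
; Its DoPickupAction adds IncreaseFuelAmount to the player's RemainingFuel, clamped between zero and MaxFuel, then plays the fuel pickup sound at the pickup's location.
; The event graph holds only disabled stub events, so the Blueprint contains no overlap detection or tick logic of its own.
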(fn `DoPickupAction`
  (bind _player_ref (`self.Player_Ref`))
  (set `/Game/Nick/BP_Player.RemainingFuel` (`KismetMathLibrary.FClamp` (+ (`/Game/Nick/BP_Player.RemainingFuel` _player_ref) (`self.IncreaseFuelAmount`)) 0.0 (`/Game/Nick/BP_Player.MaxFuel` _player_ref)) _player_ref)
  (`GameplayStatics.PlaySoundAtLocation` "/Game/Michael_Audio/Audio_Files/Fuel_Pickup.Fuel_Pickup" (`self.K2_GetActorLocation`) (struct) 1.0 1.0 0.0 null null null null))

(fn `UserConstructionScript`
  (`parent.UserConstructionScript`))