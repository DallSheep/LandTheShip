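; BP_Pickup_HealthPack is a health pack power-up that restores one point of the player's health.
; Its DoPickupAction function increments PlayerRef's Health by one only while it is below MaxHealth.
; The event graph holds only disabled default events, so this Blueprint contains no overlap detection or tick logic of its own.
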(fn `DoPickupAction`
  (bind _player_ref (`self.Player_Ref`))
  (bind _health (`/Game/Nick/BP_Player.Health` _player_ref))
  (if (< _health (`/Game/Nick/BP_Player.MaxHealth` _player_ref))
    (bind _result (`/Engine/EditorBlueprintResources/StandardMacros.IncrementInt` _health)
      (:`  `
        (set `/Game/Nick/BP_Player.Health` _result _player_ref)))))

(fn `UserConstructionScript`
  (`parent.UserConstructionScript`))